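; Knuckles is an enemy pawn that chases the player and can be killed by first-person projectiles.
; Every Tick it issues a SimpleMoveToActor through its AI controller toward the player pawn.
; A projectile hit subtracts a fixed amount of Health, destroys the pawn once none remains, and destroys the projectile.
; The logic that pitches the static mesh toward the player is disconnected and never runs.
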(event EventDestroyed)

(event EventTick
  (params (DeltaSeconds :type Float%20%28single-precision%29))
  ;[1 1 1] Move to and rotate towards player
  (AI|Navigation|SimpleMovetoActor (AI|GetAIController self) (Game|Player|GetPlayerPawn 0)))

(event Collision|EventHit
  (params (MyComp :type Primitive%20Component%20Object%20Reference) (Other :type Actor%20Object%20Reference) (OtherComp :type Primitive%20Component%20Object%20Reference) (bSelfMoved :type Boolean) (HitLocation :type Vector :default "0, 0, 0") (HitNormal :type Vector :default "0, 0, 0") (NormalImpulse :type Vector :default "0, 0, 0") (Hit :type Hit%20Result%20Structure%20%28by%20ref%29))
  (bind _asfirst_person_projectile (Utilities|Casting|CastToFirstPersonProjectile Other))
  (Variables|Default|SetHealth (- (Variables|Default|GetHealth) 1e+01))
  (if (<= (Variables|Default|GetHealth) 0.0)
    (Actor|DestroyActor))
  (Actor|DestroyActor _asfirst_person_projectile))

(fn ConstructionScript)