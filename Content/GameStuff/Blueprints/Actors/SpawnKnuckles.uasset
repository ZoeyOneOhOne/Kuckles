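; SpawnKnuckles is a spawner actor that fills a box volume with instances of the ActorToSpawn class in three growing waves.
; On BeginPlay it spawns the first wave of ten, then waves of twenty and thirty, separated by ten-second delays.
; Each instance gets a random point within the Box component's bounds and the same fixed rotation.
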(event EventBeginPlay
  (bind _box (Variables|Default|GetBox))
  (bind _box_2 (Variables|Default|GetBox))
  (bind _box_3 (Variables|Default|GetBox))
  (bind (_origin _boxextent) (Collision|GetComponentBounds _box_3))
  (bind (_origin_2 _boxextent_2) (Collision|GetComponentBounds _box))
  (bind (_origin_3 _boxextent_3) (Collision|GetComponentBounds _box_2))
  ;[1 1 1] Spawn in box
  (for _index (range 0 9)
    (Game|SpawnActorfromClass (Variables|Default|GetActorToSpawn) (Math|Transform|MakeTransform (Math|Random|RandomPointinBoundingBox _origin_2 _boxextent_2) "0.000000, 0,90.000000" "1,1,1") "Undefined" 0 0))
  (Utilities|FlowControl|Delay 1e+01)
  (for _index_2 (range 0 19)
    (Game|SpawnActorfromClass (Variables|Default|GetActorToSpawn) (Math|Transform|MakeTransform (Math|Random|RandomPointinBoundingBox _origin_3 _boxextent_3) "0.000000, 0,90.000000" "1,1,1") "Undefined" 0 0))
  (Utilities|FlowControl|Delay 1e+01)
  (for _index_3 (range 0 29)
    (Game|SpawnActorfromClass (Variables|Default|GetActorToSpawn) (Math|Transform|MakeTransform (Math|Random|RandomPointinBoundingBox _origin _boxextent) "0.000000, 0,90.000000" "1,1,1") "Undefined" 0 0)))

(fn ConstructionScript)